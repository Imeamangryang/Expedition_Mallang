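; BP_SlimeShopNPC is a shop NPC that the slime player can interact with to open the shop UI.
; Overlapping its InteractCollision reveals an interaction prompt.
; Interact sets the player's Shopping flag, prints it and shows the controller's shop widget, without calling the parent implementation.
; Leaving the collision clears the flag, hides the prompt and shop, and makes the slot widget visible.
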(event `self.ReceiveBeginPlay`
  (`SceneComponent.SetHiddenInGame` (`self.InteractUI`) true false))

(event `self.InteractCollision.OnComponentBeginOverlap`
  (params (OverlappedComponent :type "PrimitiveComponent Object Reference") (OtherActor :type "Actor Object Reference") (OtherComp :type "PrimitiveComponent Object Reference") (OtherBodyIndex :type Integer) (bFromSweep :type Boolean) (SweepResult :type "HitResult Structure (by ref)"))
  (cast `/Game/_NZW/01_Blueprints/BP_SlimePlayer` OtherActor)
  (`SceneComponent.SetHiddenInGame` (`self.InteractUI`) false false))

(event `self.InteractCollision.OnComponentEndOverlap`
  (params (OverlappedComponent :type "PrimitiveComponent Object Reference") (OtherActor :type "Actor Object Reference") (OtherComp :type "PrimitiveComponent Object Reference") (OtherBodyIndex :type Integer))
  (bind _asbp_slime_player (cast `/Game/_NZW/01_Blueprints/BP_SlimePlayer` OtherActor))
  (set `SlimePlayer.bShopping` false _asbp_slime_player)
  (`SceneComponent.SetHiddenInGame` (`self.InteractUI`) true false)
  (bind _asbp_slime_player_controller (cast `/Game/_NZW/01_Blueprints/BP_SlimePlayerController` (`GameplayStatics.GetPlayerController` 0)))
  (`Widget.SetVisibility` (`SlimePlayerController.SlotUIWidget` _asbp_slime_player_controller) "Visible")
  (`Widget.SetVisibility` (`SlimePlayerController.ShopUIWidget` _asbp_slime_player_controller) "Collapsed"))

(event `self.ReceiveActorBeginOverlap`
  (params (OtherActor :type "Actor Object Reference")))

(event `InteractableInterface.Interact`
  (bind _asbp_slime_player (cast `/Game/_NZW/01_Blueprints/BP_SlimePlayer` (`GameplayStatics.GetPlayerPawn` 0)))
  (bind _output_get (set `SlimePlayer.bShopping` true _asbp_slime_player))
  (`KismetSystemLibrary.PrintString` (`KismetStringLibrary.Conv_BoolToString` _output_get))
  (bind _asbp_slime_player_controller (cast `/Game/_NZW/01_Blueprints/BP_SlimePlayerController` (`GameplayStatics.GetPlayerController` 0)))
  (`Widget.SetVisibility` (`SlimePlayerController.ShopUIWidget` _asbp_slime_player_controller) "Visible"))

(fn `UserConstructionScript`)