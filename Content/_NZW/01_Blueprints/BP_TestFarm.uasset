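; Test slime farm actor that restores saved farm slimes and tracks which ones are inside its box.
; BeginPlay reads per-ID counts from the game instance's save and spawns BP_BaseSlime as protected at trace hits around randomized points within Radius.
; Box overlaps toggle each slime's ProtectedZone, report entry or exit through SetFarmSlimes, and re-read the counts, with debug prints.
; Spawn and SpawnItem form an alternative spawner whose only call is disconnected.
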(event `self.ReceiveBeginPlay`
  (bind _radius (`self.Radius`))
  (bind _returnvalue (`KismetMathLibrary.RandomPointInBoundingBox` (`self.K2_GetActorLocation`) (`KismetMathLibrary.MakeVector` _radius _radius)))
  (set `self.SpawnClass` "/Game/AI/BP_BaseSlime.BP_BaseSlime_C")
  (bind _asbp_slime_game_instance (cast `/Game/_NZW/01_Blueprints/BP_SlimeGameInstance` (`GameplayStatics.GetGameInstance`)))
  (bind _output_get (set `self.SlimeCounts` (`SlimePlaySaveGame.SaveFarmSlimeCounts` (`SlimeGameInstance.PlaySaveGame` _asbp_slime_game_instance))))
  (for _array_element _output_get
    (for _ (range (+ (`.Count` (break `FarmSlime` _array_element)) 1))
      (bind _outhit (`KismetSystemLibrary.LineTraceSingle` (+ _returnvalue (0.0 0.0 200.0)) (+ _returnvalue (0.0 0.0 -200.0)) "TraceTypeQuery1"))
      (bind _returnvalue_2 (`|SpawnActorFromClass` (`self.SpawnClass`) (`KismetMathLibrary.MakeTransform` (+ (`.Location` (`GameplayStatics.BreakHitResult` _outhit)) (0.0 0.0 200.0)) (`KismetMathLibrary.MakeRotator` 0.0)) "Undefined" "MultiplyWithRoot" null null))
      (bind _asaslime_actor (cast `ASlimeActor` _returnvalue_2))
      (set `ASlimeActor.ID` (break `FarmSlime` _array_element) _asaslime_actor)
      (set `ASlimeActor.bProtectedZone` true _asaslime_actor)
      (`ASlimeActor.ApplySlimeMovementImpulse` _asaslime_actor (`self.K2_GetActorLocation` _asaslime_actor) 0.0 0.0))))

(event `self.Box.OnComponentBeginOverlap`
  (params (OverlappedComponent :type "PrimitiveComponent Object Reference") (OtherActor :type "Actor Object Reference") (OtherComp :type "PrimitiveComponent Object Reference") (OtherBodyIndex :type Integer) (bFromSweep :type Boolean) (SweepResult :type "HitResult Structure (by ref)"))
  (if (`GameplayStatics.ObjectIsA` OtherActor "/Script/Expedition_Mallang.ASlimeActor")
    (bind _asaslime_actor (cast `ASlimeActor` OtherActor))
    (set `ASlimeActor.bProtectedZone` true _asaslime_actor)
    (`KismetSystemLibrary.PrintString` "슬라임 IN!!!!!" true true (struct :`R` 0.026042 :`G` 0.026042 :`B` 1.0 :`A` 1.0))
    (bind _returnvalue (`VacuumableInterface.GetID` _asaslime_actor))
    (bind _asbp_slime_game_instance (cast `/Game/_NZW/01_Blueprints/BP_SlimeGameInstance` (`GameplayStatics.GetGameInstance`)))
    (`SlimeGameInstance.SetFarmSlimes` _asbp_slime_game_instance _returnvalue true)
    (set `self.SlimeCounts` (`SlimePlaySaveGame.SaveFarmSlimeCounts` (`SlimeGameInstance.PlaySaveGame` _asbp_slime_game_instance)))))

(event `self.Box.OnComponentEndOverlap`
  (params (OverlappedComponent :type "PrimitiveComponent Object Reference") (OtherActor :type "Actor Object Reference") (OtherComp :type "PrimitiveComponent Object Reference") (OtherBodyIndex :type Integer))
  (`KismetSystemLibrary.PrintString` (`KismetStringLibrary.Conv_VectorToString` (`self.K2_GetActorLocation` OtherActor)) true true (struct :`G` 0.66 :`B` 1.0 :`A` 1.0) 100.0)
  (if (`GameplayStatics.ObjectIsA` OtherActor "/Script/Expedition_Mallang.ASlimeActor")
    (bind _asaslime_actor (cast `ASlimeActor` OtherActor))
    (set `ASlimeActor.bProtectedZone` false _asaslime_actor)
    (`KismetSystemLibrary.PrintString` "슬라임  OUT!" true true (struct :`R` 1.0 :`G` 0.098958 :`B` 0.098958 :`A` 1.0))
    (bind _returnvalue (`VacuumableInterface.GetID` _asaslime_actor))
    (bind _asbp_slime_game_instance (cast `/Game/_NZW/01_Blueprints/BP_SlimeGameInstance` (`GameplayStatics.GetGameInstance`)))
    (`SlimeGameInstance.SetFarmSlimes` _asbp_slime_game_instance _returnvalue false)
    (set `self.SlimeCounts` (`SlimePlaySaveGame.SaveFarmSlimeCounts` (`SlimeGameInstance.PlaySaveGame` _asbp_slime_game_instance)))))

(fn `Spawn`
  (for _ (`self.SlimeCounts`)
    (for _ (range (`self.CurrentItemNum`) (+ (`self.MaxCount`) 1))
      (`self.SpawnItem`))))

(fn `SpawnItem`
  (bind _radius (`self.Radius`))
  (bind _returnvalue (`KismetMathLibrary.RandomPointInBoundingBox` (`self.K2_GetActorLocation`) (`KismetMathLibrary.MakeVector` _radius _radius)))
  (bind _outhit (`KismetSystemLibrary.LineTraceSingle` (+ _returnvalue (0.0 0.0 100.0)) (+ _returnvalue (0.0 0.0 -100.0)) "TraceTypeQuery1"))
  (bind _returnvalue_2 (`|SpawnActorFromClass` (`self.SpawnClass`) (`KismetMathLibrary.MakeTransform` (+ (`.Location` (`GameplayStatics.BreakHitResult` _outhit)) (0.0 0.0 50.0)) (`KismetMathLibrary.MakeRotator` 0.0)) "Undefined" "MultiplyWithRoot" null null))
  (bind _asaslime_actor (cast `ASlimeActor` _returnvalue_2))
  (`ASlimeActor.ApplySlimeMovementImpulse` _asaslime_actor (`self.K2_GetActorLocation` _asaslime_actor) 0.0 100.0))

(fn `UserConstructionScript`)