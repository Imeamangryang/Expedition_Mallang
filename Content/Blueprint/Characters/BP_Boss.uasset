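; BP_Boss is an interactable boss character that shows a widget while the SlimePlayer is inside its InteractCollision.
; The widget starts hidden, appears on overlap and hides again when the player leaves, which also makes the player controller's SlotUIWidget visible.
; Interact sets the player's movement mode to None and starts the boss's StateTree logic, which drives whatever follows.
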(event `self.ReceiveBeginPlay`
  (`SceneComponent.SetHiddenInGame` (`self.Widget`) true false))

(event `self.InteractCollision.OnComponentBeginOverlap`
  (params (OverlappedComponent :type "PrimitiveComponent Object Reference") (OtherActor :type "Actor Object Reference") (OtherComp :type "PrimitiveComponent Object Reference") (OtherBodyIndex :type Integer) (bFromSweep :type Boolean) (SweepResult :type "HitResult Structure (by ref)"))
  (cast `SlimePlayer` OtherActor)
  (`SceneComponent.SetHiddenInGame` (`self.Widget`) false false))

(event `self.InteractCollision.OnComponentEndOverlap`
  (params (OverlappedComponent :type "PrimitiveComponent Object Reference") (OtherActor :type "Actor Object Reference") (OtherComp :type "PrimitiveComponent Object Reference") (OtherBodyIndex :type Integer))
  (cast `SlimePlayer` OtherActor)
  (`SceneComponent.SetHiddenInGame` (`self.Widget`) true false)
  (bind _asbp_slime_player_controller (cast `/Game/_NZW/01_Blueprints/BP_SlimePlayerController` (`GameplayStatics.GetPlayerController` 0)))
  (`Widget.SetVisibility` (`SlimePlayerController.SlotUIWidget` _asbp_slime_player_controller) "Visible"))

(event `InteractableInterface.Interact`
  (`CharacterMovementComponent.SetMovementMode` (`Character.CharacterMovement` (`GameplayStatics.GetPlayerCharacter` 0)) "MOVE_None" 0)
  (`BrainComponent.StartLogic` (`self.StateTree`)))

(fn `UserConstructionScript`)