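; Player character Blueprint for a slime game, handling the pause menu and two hotkeys that act like debug cheats.
; Escape toggles pause, adding or removing a WBP_ResumeDialogue widget and toggling the mouse cursor; pausing also sets Game and UI input mode, which unpausing here does not revert.
; F9 spawns a BP_GreenPlort ahead of the player, and F10 calls UpdateNewbucks with a fixed amount.
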(event `Key|Escape` :paused true
  (params (Key :type "Key Structure"))
  (bind _returnvalue (`GameplayStatics.GetPlayerController` 0))
  ; 일시정지 기능
  (:`Pressed`
    (if (`GameplayStatics.IsGamePaused`)
      (`Widget.RemoveFromParent` (`self.Dialogue`))
      (`GameplayStatics.SetGamePaused` false)
      (set `PlayerController.bShowMouseCursor` false (`GameplayStatics.GetPlayerController` 0))
      (else
        (bind _returnvalue_2 (`|CreateWidget` "/Game/UI/Subwidgets/WBP_ResumeDialogue.WBP_ResumeDialogue_C" (`GameplayStatics.GetPlayerController` 0)))
        (bind _output_get (set `self.Dialogue` _returnvalue_2))
        (`UserWidget.AddToViewport` _output_get 0)
        (set `PlayerController.bShowMouseCursor` true _returnvalue)
        (`WidgetBlueprintLibrary.SetInputMode_GameAndUIEx` _returnvalue null)
        (`GameplayStatics.SetGamePaused` true)))))

(event `Key|F9`
  (params (Key :type "Key Structure"))
  (:`Pressed`
    (`|SpawnActorFromClass` "/Game/Blueprint/BP_GreenPlort.BP_GreenPlort_C" (`KismetMathLibrary.MakeTransform` (+ (`self.K2_GetActorLocation`) (* (`self.GetActorForwardVector`) 500.0))) "Undefined" "MultiplyWithRoot" null null)))

(event `Key|F10`
  (params (Key :type "Key Structure"))
  (:`Pressed`
    (`self.UpdateNewbucks` 1000)))

(fn `UserConstructionScript`)